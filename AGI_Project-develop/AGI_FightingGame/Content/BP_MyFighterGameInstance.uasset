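; Game instance for a fighting game that controls top-level flow between main menu, match, and Parasite or Nightshade win screens.
; Init starts a state machine at MainMenu, whose state-change event opens each state's map and sets input mode and cursor.
; After a short delay following each level load, it shows that state's widget, reusing the stored instance if still valid.
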(event Custom|CustomEvent_0
  (params (NewState :type String) (OldState :type String))
  (bind _returnvalue (Game|GetPlayerController 0))
  (bind _returnvalue_2 (Game|GetPlayerController 0))
  (bind _returnvalue_3 (Game|GetPlayerController 0))
  (bind _returnvalue_4 (Game|GetPlayerController 0))
  (switch string NewState
    (:MainMenu
      ;[1 1 1] Main Menu
      (Game|OpenLevel(byName) "MainMenuMap")
      (Utilities|FlowControl|Delay 0.2)
      (Game|SetGamePaused false)
      (if (Utilities|IsValid (Variables|Default|GetMainMenuScreen))
        _
        (else
          (bind _returnvalue_5 (UserInterface|CreateWidget "/Game/Widgets/MainMenu/InitialSplash.InitialSplash_C"))
          (Variables|Default|SetMainMenuScreen _returnvalue_5)))
      (UserInterface|Viewport|AddtoViewport (Variables|Default|GetMainMenuScreen) 0)
      (Input|SetInputModeUIOnly _returnvalue_3 (Variables|Default|GetMainMenuScreen) "DoNotLock")
      (Variables|/Script/Engine.PlayerController|SetbShowMouseCursor _returnvalue_3 true))
    (:InGame
      ;[1 1 1] In Game
      (Viewport|RemoveAllWidgets)
      (Game|OpenLevel(byName) "SideScrollerExampleMap")
      (Utilities|FlowControl|Delay 0.2)
      (if (Utilities|IsValid (Variables|Default|GetInGame))
        _
        (else
          (bind _returnvalue_6 (UserInterface|CreateWidget "/Game/Widgets/InGame/InGameUI.InGameUI_C"))
          (Variables|Default|SetInGame _returnvalue_6)))
      (UserInterface|Viewport|AddtoViewport (Variables|Default|GetInGame) 0)
      (Input|SetInputModeGameOnly _returnvalue_4)
      (Variables|/Script/Engine.PlayerController|SetbShowMouseCursor _returnvalue_4 false))
    (:ParasiteWin
      (Viewport|RemoveAllWidgets)
      (Game|OpenLevel(byName) "ParasiteWinMap")
      (Utilities|FlowControl|Delay 0.2)
      (if (Utilities|IsValid (Variables|Default|GetParasiteWin))
        _
        (else
          (bind _returnvalue_7 (UserInterface|CreateWidget "/Game/Widgets/WinStates/ParasiteWin.ParasiteWin_C"))
          (Variables|Default|SetParasiteWin _returnvalue_7)))
      (UserInterface|Viewport|AddtoViewport (Variables|Default|GetParasiteWin) 0)
      (Input|SetInputModeGameOnly _returnvalue)
      (Variables|/Script/Engine.PlayerController|SetbShowMouseCursor _returnvalue true))
    (:NightshadeWin
      (Viewport|RemoveAllWidgets)
      (Game|OpenLevel(byName) "NightshadeWinMap")
      (Utilities|FlowControl|Delay 0.2)
      (if (Utilities|IsValid (Variables|Default|GetNightshadeWin))
        _
        (else
          (bind _returnvalue_8 (UserInterface|CreateWidget "/Game/Widgets/WinStates/NightshadeWin.NightshadeWin_C"))
          (Variables|Default|SetNightshadeWin _returnvalue_8)))
      (UserInterface|Viewport|AddtoViewport (Variables|Default|GetNightshadeWin) 0)
      (Input|SetInputModeGameOnly _returnvalue_2)
      (Variables|/Script/Engine.PlayerController|SetbShowMouseCursor _returnvalue_2 true))))

(event EventInit
  (bind _statemachine (Variables|Default|GetStateMachine))
  (Variables|/Script/AGI_FightingGame.BasicStateMachine|SetStates _statemachine (Variables|Default|GetInitialState))
  (EventDispatchers|BindEventtoOnStateChanged _statemachine (delegate Custom|CustomEvent_0))
  (Class|BasicStateMachine|SetState _statemachine "MainMenu"))